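; BP_Pistol_CHEAT is a pistol weapon that snaps to the player character mesh's "Weapon" socket on any actor overlap.
; Shoot_Gun fires a hitscan trace on the Camera channel from the player camera out to AttackRange, with debug drawing and a gunshot sound.
; Blocking hits spawn an impact particle and sound, then apply BaseDamage to actors that can be damaged.
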(event Custom|Shoot_Gun
  (bind _returnvalue (Game|GetPlayerCameraManager 0))
  (bind _returnvalue_2 (Transformation|GetActorLocation _returnvalue))
  ;[1 1 1] Shooting (Line trace)
  (bind _outhit (Collision|LineTraceByChannel _returnvalue_2 (+ _returnvalue_2 (* (Transformation|GetActorForwardVector _returnvalue) (Variables|Default|GetattackRange))) "TraceTypeQuery2" true 0 "ForDuration"))
  (Audio|PlaySoundatLocation "/Game/SciFiWeapDark/Sound/Pistol/Wavs/PistolA_Fire01.PistolA_Fire01" _returnvalue_2 "0, 0, 0" 1.0 1.0 0.0 0 0 0)
  (if (.bblockinghit _outhit)
    (Effects|SpawnEmitteratLocation "/Game/SciFiWeapDark/FX/Particles/P_Impact_Stone_Large_Dark.P_Impact_Stone_Large_Dark" (.location _outhit) "0, 0, 0" "0.200000,0.200000,0.200000")
    (Audio|PlaySoundatLocation "/Game/SciFiWeapDark/Sound/Rifle/Wavs/Rifle_ImpactBody01.Rifle_ImpactBody01" (.location _outhit) "0, 0, 0" 1.0 1.0 0.0 0 0 0)
    (if (Variables|/Script/Engine.Actor|GetbCanBeDamaged (.hitactor _outhit))
      (Game|Damage|ApplyDamage (.hitactor _outhit) (Variables|Default|GetBase%20Damage) 0 0))))

(event Collision|EventActorBeginOverlap
  (params (OtherActor :type Actor%20Object%20Reference))
  ;[1 1 1] Pick up
  (Transformation|AttachComponentToComponent (Variables|/Script/Engine.Character|GetMesh (Game|GetPlayerCharacter 0)) "Weapon" "SnapToTarget" "SnapToTarget" "KeepRelative" true))

(fn ConstructionScript)