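; BP_Pistol is a pistol pickup that fires hitscan shots and has a cheat-powered golden variant.
; Any overlap attaches it to the player's Weapon socket, sets HasGun on the character and applies the golden material if the Cheat actor reports cheating.
; Shoot_Gun line-traces from the camera with debug drawing, plays fire and impact effects, and applies point damage to damageable actors, using the cheat damage value while cheating.
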(event Custom|Shoot_Gun
  (bind _returnvalue (Game|GetPlayerCameraManager 0))
  (bind _returnvalue_2 (Transformation|GetActorLocation _returnvalue))
  ;[1 1 1] Shooting (Line trace)
  (bind _outhit (Collision|LineTraceByChannel _returnvalue_2 (+ _returnvalue_2 (* (Transformation|GetActorForwardVector _returnvalue) (Variables|Default|GetattackRange))) "TraceTypeQuery2" true 0 "ForDuration"))
  (Audio|PlaySoundatLocation "/Game/SciFiWeapDark/Sound/Pistol/Wavs/PistolA_Fire01.PistolA_Fire01" _returnvalue_2 "0, 0, 0" 0.2 1.0 0.0 "/Game/SciFiWeapDark/Sound/Attenuation/WeaponShot_att.WeaponShot_att" 0 0)
  (if (.bBlockingHit (Collision|BreakHitResult _outhit))
    (Effects|SpawnEmitteratLocation "/Game/SciFiWeapDark/FX/Particles/P_Impact_Stone_Large_Dark.P_Impact_Stone_Large_Dark" (.Location (Collision|BreakHitResult _outhit)) "0, 0, 0" "0.200000,0.200000,0.200000")
    (Audio|PlaySoundatLocation "/Game/SciFiWeapDark/Sound/Rifle/Wavs/Rifle_ImpactBody01.Rifle_ImpactBody01" (.Location (Collision|BreakHitResult _outhit)) "0, 0, 0" 0.4 1.0 0.0 "/Game/SciFiWeapDark/Sound/Attenuation/ProjectileImpact_att.ProjectileImpact_att" 0 0)
    (if (Variables|/Script/Engine.Actor|GetbCanBeDamaged (.HitActor (Collision|BreakHitResult _outhit)))
      ;[1 1 1] Checking if cheating
      (bind _returnvalue_3 (Actor|GetActorOfClass "/Game/KitFisto/KF_Props/Cheat.Cheat_C"))
      (if (Variables|/Game/KitFisto/KF_Props/Cheat.Cheat_C|GetisCheating _returnvalue_3)
        ;[1 1 1] Cheat Damage
        (Game|Damage|ApplyPointDamage (.HitActor (Collision|BreakHitResult _outhit)) (Variables|Default|GetdamageCheat) (.TraceStart (Collision|BreakHitResult _outhit)) _outhit)
        (Development|PrintString "cheat hit")
        (else
          ;[1 1 1] Normal Damage
          (Game|Damage|ApplyPointDamage (.HitActor (Collision|BreakHitResult _outhit)) (Variables|Default|GetBase%20Damage) (.TraceStart (Collision|BreakHitResult _outhit)) _outhit)
          (Development|PrintString "normal hit"))))))

(event Collision|EventActorBeginOverlap
  (params (OtherActor :type Actor%20Object%20Reference))
  ;[1 1 1] Pick up
  (Transformation|AttachComponentToComponent (Variables|/Script/Engine.Character|GetMesh (Game|GetPlayerCharacter 0)) "Weapon" "SnapToTarget" "SnapToTarget" "KeepRelative" true)
  ;[1 1 1] Check if Pistol has been picked up
  (bind _asthird_person_character_main (Utilities|Casting|CastToThirdPersonCharacterMAIN (Game|GetPlayerCharacter 0)))
  (Variables|/Game/ODSMannequin/ThirdPersonBP/Blueprints/ThirdPersonCharacterMAIN.ThirdPersonCharacterMAIN_C|SethasGun _asthird_person_character_main true)
  ;[1 1 1] Cheating = Golden gun
  (bind _returnvalue (Actor|GetActorOfClass "/Game/KitFisto/KF_Props/Cheat.Cheat_C"))
  (if (Variables|/Game/KitFisto/KF_Props/Cheat.Cheat_C|GetisCheating _returnvalue)
    (Rendering|Material|SetMaterial (Variables|Default|GetPistol) 0 "/Game/SciFiWeapDark/Weapons/Materials/M_Pistol_Inst_Golden.M_Pistol_Inst_Golden")))

(fn ConstructionScript)